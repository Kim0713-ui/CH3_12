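; BP_Rolling is an actor that plays rolling and falling-rock audio attached to its root component.
; BeginPlay starts a loud rolling-cart sound and a falling-rock sound, then sets two looping timers that keep spawning stones-falling and falling-rock sounds.
; All sounds except the timed stones-falling one use attenuation settings.
; The Sphere overlap event is empty, leaving the player-cast and game-pause logic disconnected.
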(event `CustomEvent`
  (`GameplayStatics.SpawnSoundAttached` "/Game/Sound/Falling_Rock/freesound_community-stones-falling-6375.freesound_community-stones-falling-6375" (`self.RootComponent`) "None" (0.0 0.0 0.0) (struct) "KeepRelativeOffset" false 1.0 1.0 0.0 "/USDCore/USDDefaultAttenuation.USDDefaultAttenuation" null))

(event `CustomEvent_1`
  (`GameplayStatics.SpawnSoundAttached` "/Game/Sound/Falling_Rock/freesound_community-falling-rock-105396.freesound_community-falling-rock-105396" (`self.RootComponent`) "None" (0.0 0.0 0.0) (struct) "KeepRelativeOffset" false 1.0 1.0 0.0 "/USDCore/USDDefaultAttenuation.USDDefaultAttenuation" null))

(event `self.ReceiveBeginPlay`
  (`|ExecutionSequence`
    (:`then_0`
      (`KismetSystemLibrary.K2_SetTimerDelegate` (delegate `CustomEvent`) 5.0 true))
    (:`then_1`
      (`KismetSystemLibrary.K2_SetTimerDelegate` (delegate `CustomEvent_1`) 4.0 true))
    (:`then_2`
      (`GameplayStatics.SpawnSoundAttached` "/Game/Sound/Rolling/freesound_community-rolling-cart-002-86702.freesound_community-rolling-cart-002-86702" (`self.RootComponent`) "None" (0.0 0.0 0.0) (struct) "KeepRelativeOffset" false 6.0 1.0 0.0 "/USDCore/USDDefaultAttenuation.USDDefaultAttenuation" null))
    (:`then_3`
      (`GameplayStatics.SpawnSoundAttached` "/Game/Sound/Falling_Rock/freesound_community-falling-rock-105396.freesound_community-falling-rock-105396" (`self.RootComponent`) "None" (0.0 0.0 0.0) (struct) "KeepRelativeOffset" false 1.0 1.0 0.0 "/USDCore/USDDefaultAttenuation.USDDefaultAttenuation" null))))

(event `self.Sphere.OnComponentBeginOverlap`
  (params (OverlappedComponent :type "PrimitiveComponent Object Reference") (OtherActor :type "Actor Object Reference") (OtherComp :type "PrimitiveComponent Object Reference") (OtherBodyIndex :type Integer) (bFromSweep :type Boolean) (SweepResult :type "HitResult Structure (by ref)")))

(fn `UserConstructionScript`)